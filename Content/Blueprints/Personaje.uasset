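; Player character Blueprint that handles basic movement, mouse look and jumping.
; Forward and strafe axes feed movement input along directions derived from control rotation, with forward movement using yaw only and strafing using yaw and roll.
; Mouse axes drive controller pitch and yaw, and the Jump action triggers the built-in jump on press.
; The Run section has no working logic, and the construction script is empty.
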(event `InputAxis|Adelante/Atras`
  (params (AxisValue :type "Float (single-precision)"))
  (bind (_returnvalue_roll _returnvalue_pitch _returnvalue_yaw) (`KismetMathLibrary.BreakRotator` (`self.GetControlRotation`)))
  ;[1 1 1] Movement
  (`self.AddMovementInput` (`KismetMathLibrary.GetForwardVector` (`KismetMathLibrary.MakeRotator` 0.0 0.0 _returnvalue_yaw)) AxisValue))

(event `InputAxis|Mouse Arriba/Abajo`
  (params (AxisValue :type "Float (single-precision)"))
  ;[1 1 1] Camara
  (`self.AddControllerPitchInput` AxisValue))

(event `InputAxis|Mouse Izq/Der`
  (params (AxisValue :type "Float (single-precision)"))
  ;[1 1 1] Camara
  (`self.AddControllerYawInput` AxisValue))

(event `InputAction|Jump`
  (params (Key :type "Key Structure"))
  ;[1 1 1] Jump Action
  (:`Pressed`
    (`self.Jump`)))

(event `InputAxis|Derecha/Izquierda`
  (params (AxisValue :type "Float (single-precision)"))
  (bind (_returnvalue_roll _returnvalue_pitch _returnvalue_yaw) (`KismetMathLibrary.BreakRotator` (`self.GetControlRotation`)))
  ;[1 1 1] Movement
  (`self.AddMovementInput` (`KismetMathLibrary.GetRightVector` (`KismetMathLibrary.MakeRotator` _returnvalue_roll 0.0 _returnvalue_yaw)) AxisValue))

(event `InputAction|Run`
  (params (Key :type "Key Structure"))
  ;[1 1 1] Run
)

(fn `UserConstructionScript`)