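; Bullet is a projectile actor that damages the Player_Glasses character on overlap, apparently fired by TorrentShooter.
; Tick moves it along its forward vector at Speed, scaled by delta time, without sweeping.
; On overlap it prints a debug string, calls TakeDamage on a Player_Glasses with a fixed amount, and destroys itself.
; It passes through TorrentShooter actors and destroys itself on any other overlap.
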(event `self.ReceiveActorBeginOverlap`
  (params (OtherActor :type "Actor Object Reference"))
  (`KismetSystemLibrary.PrintString` "Character Damage")
  (bind _asplayer_glasses (cast `/Game/Character/Player/Player_Glasses` OtherActor)
    (:`then`
      (`/Game/Character/Player/Player_Glasses.takeDamage` _asplayer_glasses 20.0))
    (:`CastFailed`
      (cast `/Game/Blueprints/TorrentShooter` OtherActor
        (:`CastFailed`
          _))))
  (`self.K2_DestroyActor`))

(event `self.ReceiveTick`
  (params (DeltaSeconds :type "Float (single-precision)"))
  (`self.K2_SetActorLocation` (+ (* DeltaSeconds (* (`self.GetActorForwardVector`) (`self.speed`))) (`self.K2_GetActorLocation`))))

(fn `UserConstructionScript`)