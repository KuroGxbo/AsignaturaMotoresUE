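; Nav link proxy that makes characters jump across a smart link to its destination.
; When an agent reaches the link, it is cast to Character and launched with both XY and Z velocity overridden.
; CalculateVelocity solves the ballistic arc from agent location to destination over JumpDuration, using a hardcoded gravity constant rather than reading the world's gravity.
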(event `self.ReceiveSmartLinkReached`
  (params (Agent :type "Actor Object Reference") (Destination :type "Vector Structure (by ref)"))
  (bind `_ascarácter` (cast `Character` Agent))
  (bind _velocity (`self.CalculateVelocity` Destination (`self.K2_GetActorLocation` Agent) (`self.JumpDuration`)))
  (`Character.LaunchCharacter` `_ascarácter` _velocity true true))

(fn `CalculateVelocity`
  (params (DestinationLocation :type "Vector Structure") (StartingLocation :type "Vector Structure") (Duration :type "Float (double-precision)"))
  (returns (Velocity :type "Vector Structure"))
  (locals (InDuration :type "Float (double-precision)"))
  (bind _induration (`local.InDuration`))
  (set `local.InDuration` Duration)
  (return (`KismetMathLibrary.MakeVector` (/ (- (.x DestinationLocation) (.x StartingLocation)) _induration) (/ (- (.y DestinationLocation) (.y StartingLocation)) _induration) (/ (- (.z DestinationLocation) (+ (.z StartingLocation) (* (`KismetMathLibrary.Square` (`local.InDuration`)) -0.5 982.0))) _induration))))

(fn `UserConstructionScript`)