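; Pickup actor that awards points when the Player_Glasses character overlaps it, then spawns a row of Coin actors and destroys itself.
; A cast filters the overlapping actor before calling ScorePoints on it.
; A loop then places coins at a fixed height above the actor, stepping a running CurrentPosition offset along world Y to space them evenly.
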(event `self.ReceiveBeginPlay`
  (set `self.currentPosition` 10.0))

(event `self.ReceiveActorBeginOverlap`
  (params (OtherActor :type "Actor Object Reference"))
  (bind _asplayer_glasses (cast `/Game/Character/Player_Glasses` OtherActor))
  (`/Game/Character/Player_Glasses.scorePoints` _asplayer_glasses 10)
  (for _ (range 1 12)
    (`|SpawnActorFromClass` "/Game/Blueprints/Coin.Coin_C" (`KismetMathLibrary.MakeTransform` (`KismetMathLibrary.MakeVector` (.x (.location (`self.GetTransform`))) (+ (`self.currentPosition`) (.y (.location (`self.GetTransform`)))) (+ (.z (.location (`self.GetTransform`))) 200.0)) (.rotation (`self.GetTransform`))) "Undefined" "OverrideRootScale" null null)
    (set `self.currentPosition` (+ (`self.currentPosition`) 500.0)))
  (`self.K2_DestroyActor`))

(event `self.ReceiveTick`
  (params (DeltaSeconds :type "Float (single-precision)")))

(fn `UserConstructionScript`)