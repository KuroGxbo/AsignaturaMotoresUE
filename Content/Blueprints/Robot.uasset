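; Robot is an enemy actor that tracks the Player_Glasses character and fires Bullet actors at it when within range.
; BeginPlay caches the player and starts a looping timer that calls Shoot, which checks distance and spawns a scaled-down Bullet at the Arrow component's transform.
; Each Tick turns Base to face the player with a look-at rotation and spins the Helice propeller around its roll axis.
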(event `self.ReceiveBeginPlay`
  (bind _returnvalue (`GameplayStatics.GetActorOfClass` "/Game/Character/Player_Glasses.Player_Glasses_C"))
  (set `self.Character` _returnvalue)
  (`KismetSystemLibrary.K2_SetTimerDelegate` (delegate `EventShoot`) 2.0 true)
  (set `self.initialLocation` (`self.K2_GetActorLocation`)))

(event `EventShoot`
  (`self.Shoot`))

(event `self.ReceiveTick`
  (params (DeltaSeconds :type "Float (single-precision)"))
  (bind _base (`self.Base`))
  (bind _helice (`self.Helice`))
  (`SceneComponent.K2_SetWorldRotation` _base (`KismetMathLibrary.FindLookAtRotation` (`SceneComponent.K2_GetComponentLocation` _base) (+ (`self.K2_GetActorLocation` (`self.Character`)) (0.0 0.0 0.0))) false false)
  (`SceneComponent.K2_SetWorldRotation` _helice (`KismetMathLibrary.MakeRotator` (+ (.roll (`SceneComponent.K2_GetComponentRotation` _helice)) 10.0) (.pitch (`SceneComponent.K2_GetComponentRotation` _helice)) (.yaw (`SceneComponent.K2_GetComponentRotation` _helice))) false false))

(fn `rotation`)

(fn `Shoot`
  (bind (_returnvalue_location _returnvalue_rotation) (`KismetMathLibrary.BreakTransform` (`SceneComponent.K2_GetComponentToWorld` (`self.Arrow`))))
  (if (< (`self.GetDistanceTo` (`self.Character`)) 1000.0)
    (`|SpawnActorFromClass` "/Game/Blueprints/Bullet.Bullet_C" (`KismetMathLibrary.MakeTransform` _returnvalue_location _returnvalue_rotation (0.2 0.2 0.2)) "Undefined" "OverrideRootScale" null null)))

(fn `UserConstructionScript`)